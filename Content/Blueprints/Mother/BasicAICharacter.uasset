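; Base AI character that reacts to the player through three overlap volumes: Detected, Seen and GameOver.
; Overlap begins set the State enum, with Seen never overriding the Detected state.
; Wander picks a nearby random nav point and starts a one-time timer to an exit state.
; CheckVision only caches the player's LookAtActor: its line-of-sight checks for character and possessed objects are disconnected, and Search's rotation sweep is disabled.
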(event OnComponentBeginOverlap(Detected)
  (params (OtherActor :type Actor%20Object%20Reference) (OtherComp :type Primitive%20Component%20Object%20Reference) (OtherBodyIndex :type Integer) (bFromSweep :type Boolean) (SweepResult :type Hit%20Result%20Structure%20%28by%20ref%29))
  (if (== OtherActor (Variables|Default|GetMainChar))
    (Variables|Default|Setstate "NewEnumerator2")))

(event OnComponentEndOverlap(Detected)
  (params (OtherActor :type Actor%20Object%20Reference) (OtherComp :type Primitive%20Component%20Object%20Reference) (OtherBodyIndex :type Integer))
  (if (== OtherActor (Variables|Default|GetMainChar))
    _))

(event OnComponentBeginOverlap(Seen)
  (params (OtherActor :type Actor%20Object%20Reference) (OtherComp :type Primitive%20Component%20Object%20Reference) (OtherBodyIndex :type Integer) (bFromSweep :type Boolean) (SweepResult :type Hit%20Result%20Structure%20%28by%20ref%29))
  (if (== OtherActor (Variables|Default|GetMainChar))
    (if (!= (Variables|Default|Getstate) (Utilities|Enum|LiteralenumAiStates "NewEnumerator2"))
      (Variables|Default|Setstate "NewEnumerator3"))))

(event OnComponentEndOverlap(Seen)
  (params (OtherActor :type Actor%20Object%20Reference) (OtherComp :type Primitive%20Component%20Object%20Reference) (OtherBodyIndex :type Integer))
  (if (== OtherActor (Variables|Default|GetMainChar))
    (if (!= (Variables|Default|Getstate) (Utilities|Enum|LiteralenumAiStates "NewEnumerator2"))
      _)))

(event OnComponentBeginOverlap(GameOver)
  (params (OtherActor :type Actor%20Object%20Reference) (OtherComp :type Primitive%20Component%20Object%20Reference) (OtherBodyIndex :type Integer) (bFromSweep :type Boolean) (SweepResult :type Hit%20Result%20Structure%20%28by%20ref%29))
  (if (== OtherActor (Variables|Default|GetMainChar))
    (Variables|Default|Setstate "NewEnumerator4")))

(event OnComponentEndOverlap(GameOver)
  (params (OtherActor :type Actor%20Object%20Reference) (OtherComp :type Primitive%20Component%20Object%20Reference) (OtherBodyIndex :type Integer))
  (if (== OtherActor (Variables|Default|GetMainChar))
    _))

(fn ConstructionScript)

(fn CheckVision
  ;[1 1 1] Game Over cone
  (Variables|Default|SetLookAtActor (Variables|/Game/Blueprints/MyCharacter.MyCharacter_C|GetLookAtActor (Variables|Default|GetMainChar))))

(fn Wander
  ;[1 1 1] Search
  (Variables|Default|SetwanderPoint (Class|NavigationSystem|GetRandomPointinRadius (Transformation|GetActorLocation) 1.0 (Variables|Default|GetNavDat) "/Script/Engine.RecastFilter_UseDefaultArea"))
  (if (not (LocalVariables|GetTimerSet))
    (Utilities|Time|SetTimerbyFunctionName self "ChangeStateToExit" 1e+01)
    (LocalVariables|SetTimerSet true)))

(fn ChangeStatetoExit
  (Variables|Default|Setstate "NewEnumerator6"))

(fn Search
  (bind _returnvalue (Transformation|GetActorLocation))
  (bind _wanderpoint (Variables|Default|GetwanderPoint))
  (bind _returnvalue_2 (Math|Rotator|FindLookatRotation _returnvalue _wanderpoint))
  (bind (_pitch _yaw _roll) (Class|KismetMathLibrary|BreakRot _returnvalue_2))
  ;[1 1 1] Search
  (if false
    (if (Math|Rotator|Equal(Rotator) (Transformation|GetActorRotation) (Variables|Default|GetRotationToTarget) 0.1)
      (Variables|Default|SetRotationToTarget (Class|KismetMathLibrary|MakeRot (+ _pitch 0.0) (+ _yaw (Math|Random|RandomFloatinRange -22.0 22.0)) (+ _roll 0.0))))
    (Transformation|SetActorRotation (Math|Rotator|Lerp(Rotator) (Transformation|GetActorRotation) (Variables|Default|GetRotationToTarget) 0.15 true))))