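; Child character that watches for the player and for the object the player is possessing (the player's LookAtActor).
; Each Tick, it checks actors overlapping its vision cone and line traces from the head to confirm line of sight.
; Seeing the player prints game over; seeing an object not tagged Seen raises FearLevel and attempts to tag it.
; Back-and-forth rotation logic is present but disconnected.
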(event `self.ReceiveBeginPlay`)

(event `self.ReceiveActorBeginOverlap`
  (params (OtherActor :type "Actor Object Reference")))

(event `self.ReceiveTick`
  (params (DeltaSeconds :type "Float (single-precision)"))
  (bind _main_char_ref (`self.Main Char Ref`))
  (bind _main_char_ref_2 (`self.Main Char Ref`))
  (bind _lookatactor (`/Game/Blueprints/MyCharacter.LookAtActor` (`self.Main Char Ref`)))
  (`|ExecutionSequence`
    (:`then_0`
      ;[1 1 1] View NEEDS TO BE CLEANED UP
      (for _array_element (`PrimitiveComponent.GetOverlappingActors` (`self.Cone`) "/Script/Engine.Actor")
        (if (== _array_element _main_char_ref)
          (set `self.Trace end location` (+ (`SceneComponent.K2_GetComponentLocation` _main_char_ref) (0.0 0.0 10.0)))
          (bind _outhit (`KismetSystemLibrary.LineTraceSingle` :`Start` (`SceneComponent.K2_GetComponentLocation` (`self.Head`)) :`End` (`self.Trace end location`) :`TraceChannel` "TraceTypeQuery1" :`DrawDebugType` "ForOneFrame" :!label _label))
          (bind (_bblockinghit _time _location _normal _impactpoint _impactnormal _physmat _hitactor) (`GameplayStatics.BreakHitResult` _outhit))
          (if (== _hitactor _main_char_ref_2)
            (`KismetSystemLibrary.PrintText` "GAME OVER")
            (elif (== _hitactor (`/Game/Blueprints/MyCharacter.LookAtActor` _main_char_ref_2))
              (bind _output_get (set `self.Fear Level` (+ (`self.Fear Level`) 10.0)))
              (`KismetSystemLibrary.PrintText` (`KismetTextLibrary.Conv_DoubleToText` _output_get "HalfToEven") true true (struct :`R` 1.0 :`G` 0.068986 :`A` 1.0))
              (`KismetArrayLibrary.Array_Add` (`Actor.Tags` (`/Game/Blueprints/MyCharacter.LookAtActor` (`self.Main Char Ref`))) "Seen")))
          (elif (== _array_element _lookatactor)
            (if (not (`self.ActorHasTag` _lookatactor "Seen"))
              (set `self.Trace end location` (+ (`self.K2_GetActorLocation` _lookatactor) (0.0 0.0 10.0)))
              (goto _label))))))))

(fn `UserConstructionScript`)