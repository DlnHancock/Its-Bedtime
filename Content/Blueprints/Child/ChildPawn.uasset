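; Child pawn that watches for the main character and their possessed objects, tracking how scared the child is.
; CheckVision filters Vision overlaps, then line traces from Head to confirm sight: the character prints GameOver, while the look-at object raises FearLevel.
; It returns a scared flag plus a call flag near set fear thresholds.
; Rotate adds local rotation; events are empty, and Seen-tag and possession-input checks are unwired.
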(event `self.ReceiveBeginPlay`)

(event `self.ReceiveActorBeginOverlap`
  (params (OtherActor :type "Actor Object Reference")))

(event `self.ReceiveTick`
  (params (DeltaSeconds :type "Float (single-precision)")))

(fn `CheckVision`
  (returns (Scared :type Boolean) (Call :type Boolean))
  (bind _main_char (`self.Main Char`))
  (bind _lookatactor (`/Game/Blueprints/MyCharacter.LookAtActor` (`self.Main Char`)))
  (bind _output_get (set `self.NewVar` (`PrimitiveComponent.GetOverlappingActors` (`self.Vision`) "/Script/Engine.Actor")))
  (for _array_element _output_get
    (if (== _array_element _main_char)
      (set `self.Trace End` (+ (`SceneComponent.K2_GetComponentLocation` _main_char) (0.0 0.0 10.0)))
      (bind _outhit (`KismetSystemLibrary.LineTraceSingle` :`Start` (`SceneComponent.K2_GetComponentLocation` (`self.Head`)) :`End` (`self.Trace End`) :`TraceChannel` "TraceTypeQuery1" :`DrawDebugType` "Persistent"))
      (if (== (`.HitActor` (`GameplayStatics.BreakHitResult` _outhit)) (`self.Main Char`))
        (`KismetSystemLibrary.PrintText` "GameOver")
        (set `self.IsScared` true :!label _label)
        (else
          (bind _output_get_2 (set `self.IsScared` false :!label _label_2))))
      (return _output_get_2 (or (`KismetMathLibrary.NearlyEqual_FloatFloat` (stale _output_get_3) 25.0 1.0) (`KismetMathLibrary.NearlyEqual_FloatFloat` (stale _output_get_3) 50.0 1.0) (`KismetMathLibrary.NearlyEqual_FloatFloat` (stale _output_get_3) 75.0 1.0)))
      (elif (== _array_element _lookatactor)
        (set `self.Trace End` (+ (`self.K2_GetActorLocation` _lookatactor) (0.0 0.0 10.0)))
        (bind _outhit_2 (`KismetSystemLibrary.LineTraceSingle` :`Start` (`SceneComponent.K2_GetComponentLocation` (`self.Head`)) :`End` (`self.Trace End`) :`TraceChannel` "TraceTypeQuery1" :`DrawDebugType` "Persistent"))
        (if (== (`/Game/Blueprints/MyCharacter.LookAtActor` (`self.Main Char`)) (`.HitActor` (`GameplayStatics.BreakHitResult` _outhit_2)))
          (bind _output_get_3 (set `self.Fear Level` (+ (`self.Fear Level`) 0.5)))
          (`KismetSystemLibrary.PrintText` (`KismetTextLibrary.Conv_DoubleToText` _output_get_3 "HalfToEven"))
          (goto _label)
          (else
            (goto _label_2)))))))

(fn `Rotate`
  (params (Rotation :type "Object.Rotator Structure" :default (struct)))
  (`self.K2_AddActorLocalRotation` Rotation))

(fn `UserConstructionScript`)